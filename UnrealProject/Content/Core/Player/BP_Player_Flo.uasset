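; BP_Player_Flo is the player Blueprint for Flo, driving the player's HUD and game over screen.
; It creates the main UI widget on BeginPlay, and Tick refreshes bag and item display when the ChangedValue flag is set.
; InteractionBox overlaps with InteractiveObject components toggle the E prompt and, for Item actors, an object preview.
; A game over event adds the UMG_GameOver widget to the viewport.
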(event `self.ReceiveTick`
  (params (DeltaSeconds :type "Float (single-precision)"))
  (bind _bagvisibility (`self.BagVisibility`))
  ;[1 1 1] UI
  (if (== (`self.ChangedValue`) true)
    (`/Game/Core/UI/InGame/UMG_UserInterface.ActiveBag` (`self.PlayerUIRef`) _bagvisibility)
    (for _array_element (`self.Itens`)
      (`/Game/Core/UI/InGame/UMG_UserInterface.PickOBJ` (`self.PlayerUIRef`) _array_element _bagvisibility)
      (set `self.ChangedValue` false))))

(event `self.ReceiveBeginPlay`
  ;[1 1 1] Add UI
  (bind _returnvalue (`|CreateWidget` "/Game/Core/UI/InGame/UMG_UserInterface.UMG_UserInterface_C"))
  (bind _output_get (set `self.PlayerUIRef` _returnvalue))
  (`UserWidget.AddToViewport` _output_get 0))

(event `self.InteractionBox.OnComponentBeginOverlap`
  (params (OverlappedComponent :type "PrimitiveComponent Object Reference") (OtherActor :type "Actor Object Reference") (OtherComp :type "PrimitiveComponent Object Reference") (OtherBodyIndex :type Integer) (bFromSweep :type Boolean) (SweepResult :type "HitResult Structure (by ref)"))
  (bind _playeruiref (`self.PlayerUIRef`))
  ;[1 1 1] Overlap InteractiveObject
  (for _array_element (`self.K2_GetComponentsByClass` OtherActor "/Script/UnrealProject.InteractiveObject")
    (`/Engine/EditorBlueprintResources/StandardMacros.IsValid` _array_element
      (:`Is Valid`
        (`/Game/Core/UI/InGame/UMG_UserInterface.ActiveE` _playeruiref true)
        (bind _asitem (cast `Item` OtherActor))
        (`/Game/Core/UI/InGame/UMG_UserInterface.PreviewObj` _playeruiref (`Item.Index` _asitem) true)))))

(event `self.InteractionBox.OnComponentEndOverlap`
  (params (OverlappedComponent :type "PrimitiveComponent Object Reference") (OtherActor :type "Actor Object Reference") (OtherComp :type "PrimitiveComponent Object Reference") (OtherBodyIndex :type Integer))
  ;[1 1 1] Overlap InteractiveObject
  (for _array_element (`self.K2_GetComponentsByClass` OtherActor "/Script/UnrealProject.InteractiveObject")
    (`/Engine/EditorBlueprintResources/StandardMacros.IsValid` _array_element
      (:`Is Valid`
        (`/Game/Core/UI/InGame/UMG_UserInterface.ActiveE` (`self.PlayerUIRef`) false)
        (cast `Item` OtherActor)
        (`/Game/Core/UI/InGame/UMG_UserInterface.PreviewObj` (`self.PlayerUIRef`) 0 false)))))

(event `OnGameOver_Event_0`
  ;[1 1 1] GameOver
  (add `self.OnGameOver` (delegate `OnGameOver_Event_0`))
  (bind _returnvalue (`|CreateWidget` "/Game/Core/UI/OffGame/UMG_GameOver.UMG_GameOver_C"))
  (`UserWidget.AddToViewport` _returnvalue 0))

(fn `UserConstructionScript`)